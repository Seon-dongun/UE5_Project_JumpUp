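; BP_Cone is an actor that moves along the direction of its Arrow component, driven by a timeline.
; On BeginPlay it stores its starting location (최초위치) and plays the 이동그래프 timeline.
; Each timeline update sets the location to that start plus the arrow's forward vector scaled by the curve value (이동값) and a distance variable (이동거리), without sweeping.
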(event `self.ReceiveBeginPlay`
  (set `self.최초위치` (`self.K2_GetActorLocation`))
  (bind (_direction `_이동값`) (`Timeline|이동그래프`)
    (:`Update`
      (`self.K2_SetActorLocation` (+ (`self.최초위치`) (* (`SceneComponent.GetForwardVector` (`self.Arrow`)) (* `_이동값` (`self.이동거리`))))))))

(fn `UserConstructionScript`)