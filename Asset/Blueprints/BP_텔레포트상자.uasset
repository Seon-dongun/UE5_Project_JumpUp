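; BP_텔레포트상자 is a moving teleport box that sends overlapping actors to a destination point.
; On BeginPlay, the 이동그래프 timeline drives its offset from the start location along the Arrow's forward vector, scaled by 이동거리.
; On overlap, it waits 딜레이초 seconds, then teleports the other actor to the location and rotation of the 텔포지점 actor, with no filter on what overlaps.
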(event `self.ReceiveBeginPlay`
  (set `self.최초위치` (`self.K2_GetActorLocation`))
  (bind (_direction `_이동값`) (`Timeline|이동그래프`)
    (:`Update`
      (`self.K2_SetActorLocation` (+ (* (`SceneComponent.GetForwardVector` (`self.Arrow`)) (* `_이동값` (`self.이동거리`))) (`self.최초위치`))))))

(event `self.ReceiveActorBeginOverlap`
  (params (OtherActor :type "Actor Object Reference"))
  (bind (_returnvalue_location _returnvalue_rotation) (`KismetMathLibrary.BreakTransform` (`self.GetTransform` (`self.텔포지점`))))
  (`KismetSystemLibrary.Delay` (`self.딜레이초`))
  (`self.K2_TeleportTo` OtherActor _returnvalue_location _returnvalue_rotation))

(fn `UserConstructionScript`)