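; BP_Circle is an actor that moves along the direction of its Arrow component once play begins.
; BeginPlay stores the start location and plays the 이동그래프 timeline at the 재생속도 rate.
; Each timeline update sets the location to the start plus the Arrow's current forward vector, scaled by the curve value and the 이동거리 distance, without sweeping.
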(event `self.ReceiveBeginPlay`
  (set `self.최초위치` (`self.K2_GetActorLocation`))
  (`TimelineComponent.SetPlayRate` (`self.이동그래프`) (`self.재생속도`))
  (bind (_direction `_이동거리`) (`Timeline|이동그래프`)
    (:`Update`
      (`self.K2_SetActorLocation` (+ (`self.최초위치`) (* (`SceneComponent.GetForwardVector` (`self.Arrow`)) (* `_이동거리` (`self.이동거리`))))))))

(fn `UserConstructionScript`)